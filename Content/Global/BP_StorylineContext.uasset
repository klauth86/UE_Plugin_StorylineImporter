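; BP_StorylineContext is the Blueprint context for the Storyline dialog and quest system, bridging its events to the UI.
; On BeginPlay it creates dialog and journal widgets for the first player, passing itself to each, and adds them to the viewport.
; Dialog start, end, node and player-choice events forward state to the dialog widget.
; Quest changes send the Storyline game mode's quest entries to the journal widget.
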(event EventBIEonQuestChanged
  (bind _asstoryline_game_mode_basic (Utilities|Casting|CastToStorylineGameMode_Basic (Game|GetGameMode)))
  (Default|OnQuestChanged (Variables|Default|GetJournalWidget) (Variables|/Script/StorylineEdProj_5_03.StorylineGameMode_Basic|GetQuestEntries _asstoryline_game_mode_basic)))

(event EventBIEonStartDialog
  (Default|OnStartDialog (Variables|Default|GetDialogWidget)))

(event EventBIEonEndDialog
  (Default|OnEndDialog (Variables|Default|GetDialogWidget)))

(event EventBIEonEnterNode
  (Default|OnEnterNode (Variables|Default|GetDialogWidget) (Variables|Default|GetCurrentNode) (Variables|Default|GetSpeakingCharacter)))

(event EventBIEonLeaveNode
  (params (IsBeforePlayerChoice :type Boolean))
  (Default|OnLeaveNode (Variables|Default|GetDialogWidget) IsBeforePlayerChoice))

(event EventBIEonPlayerChoice
  (Default|OnPlayerChoice (Variables|Default|GetDialogWidget) (Variables|Default|GetPlayerChoices)))

(event EventBeginPlay
  (bind _returnvalue (UserInterface|CreateWidget "/Game/UI/BP_DialogWidget.BP_DialogWidget_C" (Game|GetPlayerController 0) self))
  (bind _output_get (Variables|Default|SetDialogWidget _returnvalue))
  (UserInterface|Viewport|AddtoViewport _output_get 0)
  (bind _returnvalue_2 (UserInterface|CreateWidget "/Game/UI/BP_JournalWidget.BP_JournalWidget_C" (Game|GetPlayerController 0) self))
  (bind _output_get_2 (Variables|Default|SetJournalWidget _returnvalue_2))
  (UserInterface|Viewport|AddtoViewport _output_get_2 0))

(fn ConstructionScript)